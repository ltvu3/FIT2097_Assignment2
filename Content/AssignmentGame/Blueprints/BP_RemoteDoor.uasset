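; BP_RemoteDoor is a door opened by an external RemoteDoorTriggered event rather than a key.
; While the player overlaps it, input is enabled, and a left click on the unopened door sends an observation text to MainCharacter.
; The trigger plays a timeline that lerps the door to zero rotation, marks it opened, and sets a dynamic material's Frequency parameter, restoring the base material after a short delay.
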(event `self.ReceiveBeginPlay`
  (set `self.Observation` "It doesn't look like this door can be opened with a key"))

(event `self.ReceiveActorBeginOverlap`
  (params (OtherActor :type "Actor Object Reference"))
  ;[1 1 1] Enable/Disable input depending if player is in trigger volume
  (cast `/Game/AssignmentGame/Blueprints/MainCharacter` (`GameplayStatics.GetPlayerCharacter` 0))
  (`self.EnableInput` (`GameplayStatics.GetPlayerController` 0)))

(event `self.ReceiveActorEndOverlap`
  (params (OtherActor :type "Actor Object Reference"))
  ;[1 1 1] Enable/Disable input depending if player is in trigger volume
  (cast `/Game/AssignmentGame/Blueprints/MainCharacter` (`GameplayStatics.GetPlayerCharacter` 0))
  (`self.DisableInput` (`GameplayStatics.GetPlayerController` 0)))

(event `Key|LeftMouseButton`
  (params (Key :type "Key Structure" :default "AnyKey"))
  (:`Pressed`
    (if (not (`self.Opened`))
      (cast `/Game/AssignmentGame/Blueprints/MainCharacter` (`GameplayStatics.GetPlayerCharacter` 0))
      (if (not false)
        (`self.SendObservationToCharacter`)))))

(event `RemoteDoorTriggered`
  (bind _door (`self.Door`))
  (bind _doormesh (`self.DoorMesh`))
  (bind (_direction _rotation) (`Timeline|DoorOpen`)
    (:`Update`
      (`SceneComponent.K2_SetRelativeRotation` _door (`KismetMathLibrary.RLerp` (`SceneComponent.RelativeRotation` _door) (`KismetMathLibrary.MakeRotator` 0.0 0.0 0.0) _rotation true) false false)
      (set `self.Opened` true)
      (bind _returnvalue (`PrimitiveComponent.CreateDynamicMaterialInstance` _doormesh 0 "/Game/AssignmentGame/Materials/DoorMat.DoorMat"))
      (`MaterialInstanceDynamic.SetScalarParameterValue` _returnvalue "Frequency" 1.0)
      (`KismetSystemLibrary.Delay` 1.0)
      (`PrimitiveComponent.SetMaterial` _doormesh 0 "/Game/AssignmentGame/Materials/DoorMat.DoorMat"))))

(fn `SendObservationToCharacter`
  (bind _asmain_character (cast `/Game/AssignmentGame/Blueprints/MainCharacter` (`GameplayStatics.GetPlayerCharacter` 0)))
  (set `/Game/AssignmentGame/Blueprints/MainCharacter.Observation` (`self.Observation`) _asmain_character)
  (`/Game/AssignmentGame/Blueprints/MainCharacter.ClearText` _asmain_character))

(fn `UserConstructionScript`)