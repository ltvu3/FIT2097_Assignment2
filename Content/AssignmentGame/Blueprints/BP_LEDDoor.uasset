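; BP_LEDDoor is a locked door with lights above it that shows a hint when the player left-clicks nearby.
; Trigger overlap toggles player input, and a click while unopened passes the Observation text to MainCharacter.
; OpenDoor swings the door with a timeline, clears the hint and briefly applies a dynamic material with altered Frequency.
; CloseDoor rotates the door through a second timeline without resetting the Opened state.
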(event `self.ReceiveBeginPlay`
  (set `self.Observation` "The door is locked. Lights sit above the door."))

(event `self.ReceiveActorBeginOverlap`
  (params (OtherActor :type "Actor Object Reference"))
  ;[1 1 1] Enable/Disable input depending if player is in trigger volume
  (cast `/Game/AssignmentGame/Blueprints/MainCharacter` (`GameplayStatics.GetPlayerCharacter` 0))
  (`self.EnableInput` (`GameplayStatics.GetPlayerController` 0)))

(event `self.ReceiveActorEndOverlap`
  (params (OtherActor :type "Actor Object Reference"))
  ;[1 1 1] Enable/Disable input depending if player is in trigger volume
  (cast `/Game/AssignmentGame/Blueprints/MainCharacter` (`GameplayStatics.GetPlayerCharacter` 0))
  (`self.DisableInput` (`GameplayStatics.GetPlayerController` 0)))

(event `Key|LeftMouseButton`
  (params (Key :type "Key Structure" :default "AnyKey"))
  (:`Pressed`
    (if (not (`self.Opened`))
      (cast `/Game/AssignmentGame/Blueprints/MainCharacter` (`GameplayStatics.GetPlayerCharacter` 0))
      (if (not false)
        (`self.SendObservationToCharacter`)))))

(event `OpenDoor`
  (bind _door (`self.Door`))
  (bind _doormesh (`self.DoorMesh`))
  (`|ExecutionSequence`
    (:`then_0`
      (bind (_direction _rotation) (`Timeline|DoorOpen`)
        (:`Update`
          (`SceneComponent.K2_SetRelativeRotation` _door (`KismetMathLibrary.RLerp` (`SceneComponent.RelativeRotation` _door) (`KismetMathLibrary.MakeRotator` 0.0 0.0 90.0) _rotation true) false false))))
    (:`then_1`
      (set `self.Opened` true)
      (set `self.Observation` "")
      (bind _returnvalue (`PrimitiveComponent.CreateDynamicMaterialInstance` _doormesh 0 "/Game/AssignmentGame/Materials/DoorMat.DoorMat"))
      (`MaterialInstanceDynamic.SetScalarParameterValue` _returnvalue "Frequency" 1.0)
      (`KismetSystemLibrary.Delay` 1.0)
      (`PrimitiveComponent.SetMaterial` _doormesh 0 "/Game/AssignmentGame/Materials/DoorMat.DoorMat"))))

(event `CloseDoor`
  (bind (_direction _rotation) (`Timeline|Timeline_0`)
    (:`Update`
      (`SceneComponent.K2_SetRelativeRotation` (`self.Door`) (`KismetMathLibrary.MakeRotator` 0.0 0.0 _rotation) false false))))

(fn `SendObservationToCharacter`
  (bind _asmain_character (cast `/Game/AssignmentGame/Blueprints/MainCharacter` (`GameplayStatics.GetPlayerCharacter` 0)))
  (set `/Game/AssignmentGame/Blueprints/MainCharacter.Observation` (`self.Observation`) _asmain_character)
  (`/Game/AssignmentGame/Blueprints/MainCharacter.ClearText` _asmain_character))

(fn `UserConstructionScript`)