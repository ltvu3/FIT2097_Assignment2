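; BP_Switch is a one-shot "U"-shaped switch that remotely triggers a door and gives the player observation text.
; Overlap begin and end enable and disable its input, and entering also sends the current observation to MainCharacter.
; The first left click calls RemoteDoorTriggered on the first BP_RemoteDoor found via GetAllActorsOfClass and sets Pushed.
; Each click updates the observation, which SendObservationToCharacter copies to the character before calling ClearText.
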(event `self.ReceiveBeginPlay`
  (set `self.Observation` "It looks like the \"U\" shape can be pushed")
  (set `self.Pushed` false))

(event `self.ReceiveActorBeginOverlap`
  (params (OtherActor :type "Actor Object Reference"))
  (`|ExecutionSequence`
    (:`then_0`
      (`self.SendObservationToCharacter`))
    (:`then_1`
      ;[1 1 1] Enable/Disable input depending if player is in trigger volume
      (cast `/Game/AssignmentGame/Blueprints/MainCharacter` (`GameplayStatics.GetPlayerCharacter` 0))
      (`self.EnableInput` (`GameplayStatics.GetPlayerController` 0)))))

(event `self.ReceiveActorEndOverlap`
  (params (OtherActor :type "Actor Object Reference"))
  ;[1 1 1] Enable/Disable input depending if player is in trigger volume
  (cast `/Game/AssignmentGame/Blueprints/MainCharacter` (`GameplayStatics.GetPlayerCharacter` 0))
  (`self.DisableInput` (`GameplayStatics.GetPlayerController` 0)))

(event `Key|LeftMouseButton`
  (params (Key :type "Key Structure" :default "AnyKey"))
  (:`Pressed`
    (if (`self.Pushed`)
      (set `self.Observation` "The button has already been pushed")
      (else
        ;[1 1 1] Cast to the door BP, so the custom event can be called
        (bind _outactors (`GameplayStatics.GetAllActorsOfClass` "/Game/AssignmentGame/Blueprints/BP_RemoteDoor.BP_RemoteDoor_C"))
        (`/Game/AssignmentGame/Blueprints/BP_RemoteDoor.RemoteDoorTriggered` (`KismetArrayLibrary.Array_Get` _outactors))
        (set `self.Observation` "You push the \"U\" down")
        (set `self.Pushed` true)))
    (`self.SendObservationToCharacter`)))

(fn `SendObservationToCharacter`
  (bind _asmain_character (cast `/Game/AssignmentGame/Blueprints/MainCharacter` (`GameplayStatics.GetPlayerCharacter` 0)))
  (set `/Game/AssignmentGame/Blueprints/MainCharacter.Observation` (`self.Observation`) _asmain_character)
  (`/Game/AssignmentGame/Blueprints/MainCharacter.ClearText` _asmain_character))

(fn `UserConstructionScript`)