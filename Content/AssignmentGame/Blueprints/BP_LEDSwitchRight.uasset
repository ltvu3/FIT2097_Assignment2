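; BP_LEDSwitchRight is a switch actor that turns on the right side of the LED lights.
; A left mouse press finds the first BP_LEDLights actor in the level and calls TurnRightOn on it.
; It then sets an observation text about pushing the "U" down and sends it to the character.
; The trigger is a raw key event, with no click or overlap check in this graph.
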(event `Key|LeftMouseButton`
  (params (Key :type "Key Structure" :default "AnyKey"))
  (:`Pressed`
    (bind _outactors (`GameplayStatics.GetAllActorsOfClass` "/Game/AssignmentGame/Blueprints/BP_LEDLights.BP_LEDLights_C"))
    (`/Game/AssignmentGame/Blueprints/BP_LEDLights.TurnRightOn` (`KismetArrayLibrary.Array_Get` _outactors))
    (set `self.Observation` "You push the \"U\" down")
    (`self.SendObservationToCharacter`)))

(fn `UserConstructionScript`
  (`parent.UserConstructionScript`))