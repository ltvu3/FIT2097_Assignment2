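; BP_Medkit is a one-time healing pickup that represents blue smoke from a copper pipe.
; Any overlap adds HealAmount to the player MainCharacter's Health, capped at 1.0, without checking which actor overlapped.
; It then destroys its particles and trigger volume and turns off the pipe's glow through a dynamic material instance.
; Finally, it passes observation text about the healing smoke to the character and calls ClearText.
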(event `self.ReceiveBeginPlay`
  (set `self.Observation` "Inhaling the blue smoke heals you slightly"))

(event `self.ReceiveActorBeginOverlap`
  (params (OtherActor :type "Actor Object Reference"))
  (bind _asmain_character (cast `/Game/AssignmentGame/Blueprints/MainCharacter` (`GameplayStatics.GetPlayerCharacter` 0)))
  (bind _returnvalue (+ (`/Game/AssignmentGame/Blueprints/MainCharacter.Health` _asmain_character) (`self.HealAmount`)))
  (if (>= _returnvalue 1.0)
    (set `/Game/AssignmentGame/Blueprints/MainCharacter.Health` 1.0 _asmain_character)
    (else
      (set `/Game/AssignmentGame/Blueprints/MainCharacter.Health` _returnvalue _asmain_character)))
  (`ActorComponent.K2_DestroyComponent` (`self.ParticleSystem`))
  (`ActorComponent.K2_DestroyComponent` (`self.TriggerVolume`))
  (bind _returnvalue_2 (`PrimitiveComponent.CreateDynamicMaterialInstance` (`self.MainPipe`) 0 "/Game/AssignmentGame/Materials/CopperItem.CopperItem"))
  (`MaterialInstanceDynamic.SetScalarParameterValue` _returnvalue_2 "Glow" 0.0)
  (`self.SendObservationToPlayer`))

(fn `SendObservationToPlayer`
  (bind _asmain_character (cast `/Game/AssignmentGame/Blueprints/MainCharacter` (`GameplayStatics.GetPlayerCharacter` 0)))
  (set `/Game/AssignmentGame/Blueprints/MainCharacter.Observation` (`self.Observation`) _asmain_character)
  (`/Game/AssignmentGame/Blueprints/MainCharacter.ClearText` _asmain_character))

(fn `UserConstructionScript`)