(event `self.ReceiveBeginPlay`
  (set `self.Observation` ""))

(event `self.ReceiveActorBeginOverlap`
  (params (OtherActor :type "Actor Object Reference"))
  (`|ExecutionSequence`
    (:`then_0`
      (`self.SendObservationToPlayer`))
    (:`then_1`
      ;[1 1 1] Enable/Disable input depending if player is in trigger volume
      (cast `/Game/AssignmentGame/Blueprints/MainCharacter` (`GameplayStatics.GetPlayerCharacter` 0))
      (`self.EnableInput` (`GameplayStatics.GetPlayerController` 0)))))

(event `self.ReceiveActorEndOverlap`
  (params (OtherActor :type "Actor Object Reference"))
  ;[1 1 1] Enable/Disable input depending if player is in trigger volume
  (cast `/Game/AssignmentGame/Blueprints/MainCharacter` (`GameplayStatics.GetPlayerCharacter` 0))
  (`self.DisableInput` (`GameplayStatics.GetPlayerController` 0)))

(event `Key|LeftMouseButton`
  (params (Key :type "Key Structure"))
  (:`Pressed`
    (if (not (`self.Taken`))
      (`self.KeyTaken`)
      (`self.SendObservationToPlayer`)
      (set `self.Taken` true)
      (set `self.Observation` ""))))

(fn `KeyTaken`
  ;[1 1 1] Hides key mesh
  (`self.SetActorHiddenInGame` true)
  ;[1 1 1] Tell player class that they now have the key
  (bind _asmain_character (cast `/Game/AssignmentGame/Blueprints/MainCharacter` (`GameplayStatics.GetPlayerCharacter` 0)))
  (set `/Game/AssignmentGame/Blueprints/MainCharacter.hasKey` true _asmain_character)
  ;[1 1 1] Update observation for UI
  (set `self.Observation` "You take the key"))

(fn `SendObservationToPlayer`
  (bind _asmain_character (cast `/Game/AssignmentGame/Blueprints/MainCharacter` (`GameplayStatics.GetPlayerCharacter` 0)))
  (set `/Game/AssignmentGame/Blueprints/MainCharacter.Observation` (`self.Observation`) _asmain_character)
  (`/Game/AssignmentGame/Blueprints/MainCharacter.ClearText` _asmain_character))

(fn `UserConstructionScript`)