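; BP_LastDoorTrigger is an overlap trigger for the last door that shuts it and changes the player character's state.
; Any actor overlap closes the first BP_LEDDoor found in the level.
; It then finds the first MainCharacter, zeroes its DamageRate, calls UpdateTimer, resets walk speed to WalkValue and disables sprint.
; Both targets come from GetAllActorsOfClass, with no check on the overlapping actor.
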(event `self.ReceiveActorBeginOverlap`
  (params (OtherActor :type "Actor Object Reference"))
  (bind _outactors (`GameplayStatics.GetAllActorsOfClass` "/Game/AssignmentGame/Blueprints/BP_LEDDoor.BP_LEDDoor_C"))
  (`/Game/AssignmentGame/Blueprints/BP_LEDDoor.CloseDoor` (`KismetArrayLibrary.Array_Get` _outactors))
  (bind _outactors_2 (`GameplayStatics.GetAllActorsOfClass` "/Game/AssignmentGame/Blueprints/MainCharacter.MainCharacter_C"))
  (bind _item (`KismetArrayLibrary.Array_Get` _outactors_2))
  (set `/Game/AssignmentGame/Blueprints/MainCharacter.DamageRate` 0.0 _item)
  (`/Game/AssignmentGame/Blueprints/MainCharacter.UpdateTimer` _item)
  (set `CharacterMovementComponent.MaxWalkSpeed` (`/Game/AssignmentGame/Blueprints/MainCharacter.WalkValue` _item) (`Character.CharacterMovement` _item))
  (set `/Game/AssignmentGame/Blueprints/MainCharacter.disableSprint` true _item))

(fn `UserConstructionScript`)