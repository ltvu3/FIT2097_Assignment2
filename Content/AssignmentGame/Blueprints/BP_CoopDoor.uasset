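; BP_CoopDoor is a door actor with two pressure-plate triggers, either of which swings it open.
; Each trigger's begin overlap sets its plate flag and plays the shared DoorOpening timeline, which drives the Door's yaw.
; On end overlap the flag clears, and the timeline reverses only if the other plate is also unoccupied.
; Overlaps accept any actor, and each plate tracks occupancy as a single boolean rather than a count.
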(event `self.Trigger1.OnComponentBeginOverlap`
  (params (OverlappedComponent :type "PrimitiveComponent Object Reference") (OtherActor :type "Actor Object Reference") (OtherComp :type "PrimitiveComponent Object Reference") (OtherBodyIndex :type Integer) (bFromSweep :type Boolean) (SweepResult :type "HitResult Structure (by ref)"))
  (set `self.onPlate1` true)
  (bind (_direction _z_rotation) (`Timeline|DoorOpening` :!label _label)
    (:`Update`
      (`SceneComponent.K2_SetRelativeRotation` (`self.Door`) (`KismetMathLibrary.MakeRotator` 0.0 0.0 _z_rotation) false false))))

(event `self.Trigger2.OnComponentBeginOverlap`
  (params (OverlappedComponent :type "PrimitiveComponent Object Reference") (OtherActor :type "Actor Object Reference") (OtherComp :type "PrimitiveComponent Object Reference") (OtherBodyIndex :type Integer) (bFromSweep :type Boolean) (SweepResult :type "HitResult Structure (by ref)"))
  (set `self.onPlate2` true)
  (goto _label))

(event `self.Trigger1.OnComponentEndOverlap`
  (params (OverlappedComponent :type "PrimitiveComponent Object Reference") (OtherActor :type "Actor Object Reference") (OtherComp :type "PrimitiveComponent Object Reference") (OtherBodyIndex :type Integer))
  (set `self.onPlate1` false)
  (if (not (`self.onPlate2`))
    (goto _label :!via `Reverse`)))

(event `self.Trigger2.OnComponentEndOverlap`
  (params (OverlappedComponent :type "PrimitiveComponent Object Reference") (OtherActor :type "Actor Object Reference") (OtherComp :type "PrimitiveComponent Object Reference") (OtherBodyIndex :type Integer))
  (set `self.onPlate2` false)
  (if (not (`self.onPlate1`))
    (goto _label :!via `Reverse`)))

(fn `UserConstructionScript`)