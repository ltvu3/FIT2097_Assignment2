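; Fuse box puzzle that takes the player's fuse and opens a BP_FuseDoor once the fuse is rotated to the top position.
; Overlap toggles input, and left click installs a carried fuse, opens the FuseBoxUIWidget, or sends observation text to MainCharacter.
; RotateCounter and RotateClockwise turn the fuse pivot in quarter steps by playing four shared timelines forward or reversed.
; Timeline updates track position using a direction flag and set Done at the top.
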(event `self.ReceiveBeginPlay`
  (`SceneComponent.SetVisibility` (`self.mainfuse`) false false))

(event `self.ReceiveActorBeginOverlap`
  (params (OtherActor :type "Actor Object Reference"))
  (`|ExecutionSequence`
    (:`then_1`
      ;[1 1 1] Enable/Disable input depending if player is in trigger volume
      (cast `/Game/AssignmentGame/Blueprints/MainCharacter` (`GameplayStatics.GetPlayerCharacter` 0))
      (`self.EnableInput` (`GameplayStatics.GetPlayerController` 0)))))

(event `self.ReceiveActorEndOverlap`
  (params (OtherActor :type "Actor Object Reference"))
  ;[1 1 1] Enable/Disable input depending if player is in trigger volume
  (cast `/Game/AssignmentGame/Blueprints/MainCharacter` (`GameplayStatics.GetPlayerCharacter` 0))
  (`self.DisableInput` (`GameplayStatics.GetPlayerController` 0)))

(event `Key|LeftMouseButton`
  (params (Key :type "Key Structure" :default "AnyKey"))
  (bind _fuzeboxuireference (`self.FuzeBoxUIReference`))
  (:`Pressed`
    (bind _asmain_character (cast `/Game/AssignmentGame/Blueprints/MainCharacter` (`GameplayStatics.GetPlayerCharacter` 0)))
    (if (`/Game/AssignmentGame/Blueprints/MainCharacter.hasFuse` _asmain_character)
      (`SceneComponent.SetVisibility` (`self.mainfuse`) true false)
      (set `self.fuseInstalled` true)
      (bind _asmain_character_2 (cast `/Game/AssignmentGame/Blueprints/MainCharacter` (`GameplayStatics.GetPlayerCharacter` 0)))
      (set `/Game/AssignmentGame/Blueprints/MainCharacter.hasFuse` false _asmain_character_2)
      (set `self.Observation` "You place the fuse in the fusebox")
      (`self.SendObservationToCharacter`)
      (elif (`self.fuseInstalled`)
        (if (not (`self.done`))
          (`/Engine/EditorBlueprintResources/StandardMacros.IsValid` (`self.FuzeBoxUIReference`)
            (:`Is Valid`
              _)
            (:`Is Not Valid`
              (bind _returnvalue (`|CreateWidget` "/Game/AssignmentGame/UI/FuseBoxUIWidget.FuseBoxUIWidget_C"))
              (set `self.FuzeBoxUIReference` _returnvalue)))
          (`WidgetBlueprintLibrary.SetInputMode_UIOnlyEx` (`GameplayStatics.GetPlayerController` 0) _fuzeboxuireference)
          (`UserWidget.AddToViewport` _fuzeboxuireference 0))
        (else
          (`self.SendObservationToCharacter`))))))

(event `RotateCounter`
  (bind _rotatingcounter (`self.RotatingCounter`))
  (set `self.RotatingCounter` true)
  (switch `int` (`self.mainFusePosition`)
    (:`0`
      (bind (_direction _0_to__90) (`Timeline|RotTopToLeft` :!via `PlayFromStart` :!label _label)
        (:`Update`
          (`SceneComponent.K2_SetRelativeRotation` (`self.mainfusepivot`) (`KismetMathLibrary.MakeRotator` _0_to__90) false false)
          (if _rotatingcounter
            (set `self.mainFusePosition` 3)
            (else
              (set `self.mainFusePosition` 0)
              (set `self.done` true :!label _label_2)
              (bind _outactors (`GameplayStatics.GetAllActorsOfClass` "/Game/AssignmentGame/Blueprints/BP_FuseDoor.BP_FuseDoor_C"))
              (`KismetSystemLibrary.Delay` 1.0)
              (`/Game/AssignmentGame/Blueprints/BP_FuseDoor.RemoteDoorTriggered` (`KismetArrayLibrary.Array_Get` _outactors)))))))
    (:`1`
      (bind (_direction_2 _90_to_0) (`Timeline|RotRIghtToTop` :!via `PlayFromStart` :!label _label_3)
        (:`Update`
          (`SceneComponent.K2_SetRelativeRotation` (`self.mainfusepivot`) (`KismetMathLibrary.MakeRotator` _90_to_0) false false)
          (if _rotatingcounter
            (set `self.mainFusePosition` 0)
            (goto _label_2)
            (else
              (set `self.mainFusePosition` 1))))))
    (:`2`
      (bind (_direction_3 _test) (`Timeline|RotBotToRight` :!via `PlayFromStart` :!label _label_4)
        (:`Update`
          (`SceneComponent.K2_SetRelativeRotation` (`self.mainfusepivot`) (`KismetMathLibrary.MakeRotator` _test) false false)
          (if _rotatingcounter
            (set `self.mainFusePosition` 1)
            (else
              (set `self.mainFusePosition` 2))))))
    (:`3`
      (bind (_direction_4 __90_to__180) (`Timeline|RotLeftToBot` :!via `PlayFromStart` :!label _label_5)
        (:`Update`
          (`SceneComponent.K2_SetRelativeRotation` (`self.mainfusepivot`) (`KismetMathLibrary.MakeRotator` __90_to__180) false false)
          (if _rotatingcounter
            (set `self.mainFusePosition` 2)
            (else
              (set `self.mainFusePosition` 3))))))))

(event `RotateClockwise`
  (set `self.RotatingCounter` false)
  (switch `int` (`self.mainFusePosition`)
    (:`0`
      (goto _label_3 :!via `ReverseFromEnd`))
    (:`1`
      (goto _label_4 :!via `ReverseFromEnd`))
    (:`2`
      (goto _label_5 :!via `ReverseFromEnd`))
    (:`3`
      (goto _label :!via `ReverseFromEnd`))))

(fn `SendObservationToCharacter`
  (bind _asmain_character (cast `/Game/AssignmentGame/Blueprints/MainCharacter` (`GameplayStatics.GetPlayerCharacter` 0)))
  (set `/Game/AssignmentGame/Blueprints/MainCharacter.Observation` (`self.Observation`) _asmain_character)
  (`/Game/AssignmentGame/Blueprints/MainCharacter.ClearText` _asmain_character))

(fn `UserConstructionScript`)