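; BP_LEDLights is a three-light puzzle piece that opens an LED door once the left, middle and right lights are all on.
; Each Turn event toggles its light between the base LED material and a green emissive dynamic instance.
; All toggles share a short retriggerable delay before CheckIfAllLightsOn latches OpenDoor, which is never reset.
; While latched, it calls OpenDoor on the first BP_LEDDoor found in the level.
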(event `self.ReceiveBeginPlay`)

(event `TurnLeftOn`
  (bind _leftlight (`self.leftLight`))
  (if (`self.leftLightOn`)
    (`PrimitiveComponent.SetMaterial` _leftlight 0 "/Game/AssignmentGame/Materials/LEDMat.LEDMat")
    (set `self.leftLightOn` false)
    (else
      (bind _returnvalue (`PrimitiveComponent.CreateDynamicMaterialInstance` _leftlight 0 "/Game/AssignmentGame/Materials/LEDMat.LEDMat"))
      (bind _output_get (set `self.LEDLightMatON` _returnvalue))
      (`MaterialInstanceDynamic.SetVectorParameterValue` _output_get "EmissiveColour" (`self.Green`))
      (set `self.leftLightOn` true)))
  (`KismetSystemLibrary.RetriggerableDelay` 0.2 :!label _label)
  (`self.CheckIfAllLightsOn`)
  (if (`self.openDoor`)
    (bind _outactors (`GameplayStatics.GetAllActorsOfClass` "/Game/AssignmentGame/Blueprints/BP_LEDDoor.BP_LEDDoor_C"))
    (`/Game/AssignmentGame/Blueprints/BP_LEDDoor.OpenDoor` (`KismetArrayLibrary.Array_Get` _outactors))))

(event `TurnMiddleOn`
  (bind _middlelight (`self.middleLight`))
  (if (`self.middleLightOn`)
    (`PrimitiveComponent.SetMaterial` _middlelight 0 "/Game/AssignmentGame/Materials/LEDMat.LEDMat")
    (set `self.middleLightOn` false)
    (goto _label)
    (else
      (bind _returnvalue (`PrimitiveComponent.CreateDynamicMaterialInstance` _middlelight 0 "/Game/AssignmentGame/Materials/LEDMat.LEDMat"))
      (bind _output_get (set `self.LEDLightMatON` _returnvalue))
      (`MaterialInstanceDynamic.SetVectorParameterValue` _output_get "EmissiveColour" (`self.Green`))
      (set `self.middleLightOn` true)
      (goto _label))))

(event `TurnRightOn`
  (bind _rightlight (`self.rightLight`))
  (if (`self.RightLightOn`)
    (`PrimitiveComponent.SetMaterial` _rightlight 0 "/Game/AssignmentGame/Materials/LEDMat.LEDMat")
    (set `self.RightLightOn` false)
    (goto _label)
    (else
      (bind _returnvalue (`PrimitiveComponent.CreateDynamicMaterialInstance` _rightlight 0 "/Game/AssignmentGame/Materials/LEDMat.LEDMat"))
      (bind _output_get (set `self.LEDLightMatON` _returnvalue))
      (`MaterialInstanceDynamic.SetVectorParameterValue` _output_get "EmissiveColour" (`self.Green`))
      (set `self.RightLightOn` true)
      (goto _label))))

(fn `CheckIfAllLightsOn`
  (if (and (`self.leftLightOn`) (`self.middleLightOn`) (`self.RightLightOn`))
    (set `self.openDoor` true)))

(fn `UserConstructionScript`)