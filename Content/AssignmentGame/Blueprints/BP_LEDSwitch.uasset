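; BP_LEDSwitch is an interactable "U"-shaped switch that turns on the LED lights.
; Overlap events toggle the actor's player input, so left click works while the player is in its trigger volume.
; A click calls TurnLeftOn and TurnRightOn on the first BP_LEDLights found in the level.
; On overlap and click, it passes observation text to MainCharacter and calls its ClearText.
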(event `self.ReceiveBeginPlay`
  (set `self.Observation` "It looks like the \"U\" shape can be pushed"))

(event `self.ReceiveActorBeginOverlap`
  (params (OtherActor :type "Actor Object Reference"))
  (`|ExecutionSequence`
    (:`then_0`
      (`self.SendObservationToCharacter`))
    (:`then_1`
      ;[1 1 1] Enable/Disable input depending if player is in trigger volume
      (cast `/Game/AssignmentGame/Blueprints/MainCharacter` (`GameplayStatics.GetPlayerCharacter` 0))
      (`self.EnableInput` (`GameplayStatics.GetPlayerController` 0)))))

(event `self.ReceiveActorEndOverlap`
  (params (OtherActor :type "Actor Object Reference"))
  ;[1 1 1] Enable/Disable input depending if player is in trigger volume
  (cast `/Game/AssignmentGame/Blueprints/MainCharacter` (`GameplayStatics.GetPlayerCharacter` 0))
  (`self.DisableInput` (`GameplayStatics.GetPlayerController` 0)))

(event `Key|LeftMouseButton`
  (params (Key :type "Key Structure" :default "AnyKey"))
  (:`Pressed`
    (bind _outactors (`GameplayStatics.GetAllActorsOfClass` "/Game/AssignmentGame/Blueprints/BP_LEDLights.BP_LEDLights_C"))
    (bind _item (`KismetArrayLibrary.Array_Get` _outactors))
    (`/Game/AssignmentGame/Blueprints/BP_LEDLights.TurnLeftOn` _item)
    (`/Game/AssignmentGame/Blueprints/BP_LEDLights.TurnRightOn` _item)
    (set `self.Observation` "You push the \"U\" down")
    (`self.SendObservationToCharacter`)))

(fn `SendObservationToCharacter`
  (bind _asmain_character (cast `/Game/AssignmentGame/Blueprints/MainCharacter` (`GameplayStatics.GetPlayerCharacter` 0)))
  (set `/Game/AssignmentGame/Blueprints/MainCharacter.Observation` (`self.Observation`) _asmain_character)
  (`/Game/AssignmentGame/Blueprints/MainCharacter.ClearText` _asmain_character))

(fn `UserConstructionScript`)